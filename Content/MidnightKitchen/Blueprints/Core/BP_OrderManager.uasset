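; Order manager actor for a kitchen game that runs the customer loop: spawn, wait, serve or lose patience.
; Picks a random customer and recipe from DataTables and drives a patience bar widget from a Tick countdown.
; Delivered ingredients complete orders as Good; debug keys force Perfect, Good or Burnt, which resets patience to half.
; Serving or expiry spawns the next customer after a delay; tips and penalties are only printed.
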(event Custom|SpawnNextCustomer
  (Utilities|Array|Clear (Variables|Default|GetDeliveredIngredients))
  (bind _outrownames (DataTable|GetDataTableRowNames "/Game/MidnightKitchen/DataTables/DT_Customers.DT_Customers"))
  (bind _returnvalue (Utilities|GetDataTableRow "/Game/MidnightKitchen/DataTables/DT_Customers.DT_Customers" (.OutItem (Utilities|Array|Random _outrownames)))
    (:then
      (Variables|Default|SetCurrentCustomer _returnvalue)
      (bind _output_get (Variables|Default|SetMaxPatience (* (.BasePatience (Utilities|Struct|BreakS_CustomerData _returnvalue)) (Variables|Default|GetPatienceMultiplier))))
      (Variables|Default|SetRemainingPatience _output_get)
      (Variables|Default|SetbCustomerWaiting true)
      (Default|SetCustomer (Variables|Default|GetPatienceWidget) (.DisplayName (Utilities|Struct|BreakS_CustomerData (Variables|Default|GetCurrentCustomer))))
      (Development|PrintText (Utilities|Text|ToText(String) (Utilities|String|Append (Utilities|String|ToString(Text) (.DisplayName (Utilities|Struct|BreakS_CustomerData _returnvalue))) " geldi, sabır:" (Utilities|String|ToString(Float) (.BasePatience (Utilities|Struct|BreakS_CustomerData _returnvalue))) " sn")) true true "(R=0.000000,G=0.660000,B=1.000000,A=1.000000)" 5.0)
      (bind _outrownames_2 (DataTable|GetDataTableRowNames "/Game/MidnightKitchen/DataTables/DT_Recipes.DT_Recipes"))
      (bind _output_get_2 (Variables|Default|SetCurrentRecipeId (.OutItem (Utilities|Array|Random _outrownames_2))))
      (bind _returnvalue_2 (Utilities|GetDataTableRow "/Game/MidnightKitchen/DataTables/DT_Recipes.DT_Recipes" _output_get_2)
        (:then
          (bind _output_get_3 (Variables|Default|SetCurrentRecipe _returnvalue_2))
          (Default|SetOrder (Variables|Default|GetPatienceWidget) (.DisplayName (Utilities|Struct|BreakS_RecipeData _output_get_3))))
        (:RowNotFound
          (Development|PrintString "Tarif bulunamadı"))))
    (:RowNotFound
      (Development|PrintString "Bulunamadı"))))

(event Custom|DeliverIngredient
  (params (IngredientId :type Name))
  (bind _currentrecipe (Variables|Default|GetCurrentRecipe))
  (bind _ingredients (Utilities|Struct|BreakS_RecipeData _currentrecipe))
  (if (Utilities|Array|ContainsItem _ingredients IngredientId)
    (Utilities|Array|AddUnique (Variables|Default|GetDeliveredIngredients) IngredientId)
    (if (== (Utilities|Array|Length (Variables|Default|GetDeliveredIngredients)) (Utilities|Array|Length _ingredients))
      (CallFunction|ServeOrder "NewEnumerator1")
      (else
        (Development|PrintString "Güzel, devam")))
    (else
      (Development|PrintString "Yanlış malzeme!"))))

(event Custom|OnPatienceExpired
  (bind _currentcustomer (Variables|Default|GetCurrentCustomer))
  (bind (_displayname _basepatience _reputationpenalty _healthpenalty _earningspenaltypercent) (Utilities|Struct|BreakS_CustomerData _currentcustomer))
  (Development|PrintText (Utilities|Text|FormatText "{Ad} sabrını kaybetti! İtibar -{Itibar}, Sağlık -{Saglik}, Kazanç -%{Kazanc}" _displayname _reputationpenalty _healthpenalty _earningspenaltypercent) true true "(R=0.000000,G=0.660000,B=1.000000,A=1.000000)" 5.0)
  (Utilities|FlowControl|Delay 2.0)
  (CallFunction|SpawnNextCustomer))

(event Custom|ServeOrder
  (params (Quality :type E_DishQuality%20Enum :default "NewEnumerator0"))
  (if true
    (switch Utilities|FlowControl|Switch|SwitchonE_DishQuality Quality
      (:NewEnumerator0
        (Development|PrintText "\"Mükemmel servis! Bahşiş +%50\"")
        (Variables|Default|SetbCustomerWaiting false :!label _label)
        (Utilities|FlowControl|Delay 2.0)
        (CallFunction|SpawnNextCustomer))
      (:NewEnumerator1
        (Development|PrintText "\"İyi servis: standart ödeme\"")
        (goto _label))
      (:NewEnumerator2
        (Variables|Default|SetRemainingPatience (* (Variables|Default|GetMaxPatience) 0.5))
        (Development|PrintText "\"Yanık! Müşteri geri çevirdi, sabır -%50\"")))))

(event EventBeginPlay
  (Development|PrintString "Başladı")
  (bind _returnvalue (UserInterface|CreateWidget "/Game/MidnightKitchen/WBP_PatienceBar.WBP_PatienceBar_C"))
  (bind _output_get (Variables|Default|SetPatienceWidget _returnvalue))
  (UserInterface|Viewport|AddtoViewport _output_get 0)
  (Input|EnableInput (Game|GetPlayerController 0))
  (CallFunction|SpawnNextCustomer))

(event Collision|EventActorBeginOverlap
  (params (OtherActor :type Actor%20Object%20Reference)))

(event EventTick
  (params (DeltaSeconds :type Float%20%28single-precision%29))
  (Default|SetPatience (Variables|Default|GetPatienceWidget) (/ (Variables|Default|GetRemainingPatience) (Variables|Default|GetMaxPatience)))
  (if (Variables|Default|GetbCustomerWaiting)
    (bind _output_get (Variables|Default|SetRemainingPatience (- (Variables|Default|GetRemainingPatience) DeltaSeconds)))
    (if (<= _output_get 0.0)
      (CallFunction|OnPatienceExpired))))

(event Input|KeyboardEvents|DebugKey1
  (params (Key :type Key%20Structure :default "None") (ActionValue :type Input%20Action%20Value%20Structure))
  (:Pressed
    (CallFunction|ServeOrder "NewEnumerator0")))

(event Input|KeyboardEvents|DebugKey2
  (params (Key :type Key%20Structure :default "None") (ActionValue :type Input%20Action%20Value%20Structure))
  (:Pressed
    (CallFunction|ServeOrder "NewEnumerator1")))

(event Input|KeyboardEvents|DebugKey3
  (params (Key :type Key%20Structure :default "None") (ActionValue :type Input%20Action%20Value%20Structure))
  (:Pressed
    (CallFunction|ServeOrder "NewEnumerator2")))

(fn ConstructionScript)