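; BP_Ingredient is a clickable, draggable ingredient actor that the player drops on serving spots to fill orders.
; On construction it loads its row from DT_Ingredients by IngredientId and labels itself with the display name.
; While dragged, it ignores Visibility traces and follows the cursor hit point each Tick.
; Released over an actor tagged "Servis", it reports its ID to BP_OrderManager and returns to its start location.
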(event EventBeginPlay
  (Variables|Default|SetStartLocation (Transformation|GetActorLocation)))

(event Collision|EventActorBeginOverlap
  (params (OtherActor :type Actor%20Object%20Reference)))

(event MouseInput|EventActorOnClicked
  (params (ButtonPressed :type Key%20Structure :default "None"))
  (Variables|Default|SetbIsDragging true)
  (Collision|SetCollisionResponsetoChannel (Variables|Components|GetMesh) "ECC_Visibility" "ECR_Ignore"))

(event EventTick
  (params (DeltaSeconds :type Float%20%28single-precision%29))
  (bind _returnvalue (Game|GetPlayerController 0))
  (bind _hitresult (Game|Player|GetHitResultUnderCursorbyChannel _returnvalue "TraceTypeQuery1" true))
  (bind (_bblockinghit _binitialoverlap _time _distance _location _impactpoint _normal _impactnormal _physmat _hitactor) (Collision|BreakHitResult _hitresult))
  (if (Variables|Default|GetbIsDragging)
    (if (Game|Player|IsInputKeyDown _returnvalue "LeftMouseButton")
      (Transformation|SetActorLocation (+ (.Location (Collision|BreakHitResult (.HitResult (Game|Player|GetHitResultUnderCursorbyChannel _returnvalue "TraceTypeQuery1" true)))) "0.000000,0.000000,30.000000") false false)
      (else
        (Variables|Default|SetbIsDragging false)
        (Transformation|SetActorLocation (+ _location "0.000000,0.000000,8.000000") false false)
        (if (Actor|ActorHasTag _hitactor "Servis")
          (bind _returnvalue_2 (Actor|GetActorOfClass "/Game/MidnightKitchen/Blueprints/Core/BP_OrderManager.BP_OrderManager_C"))
          (Default|DeliverIngredient _returnvalue_2 (Variables|Default|GetIngredientId))
          (Transformation|SetActorLocation (Variables|Default|GetStartLocation) false false)
          (Collision|SetCollisionResponsetoChannel (Variables|Components|GetMesh) "ECC_Visibility" "ECR_Block" :!label _label))))
    (else
      (goto _label))))

(fn ConstructionScript
  (bind _returnvalue (Utilities|GetDataTableRow "/Game/MidnightKitchen/DataTables/DT_Ingredients.DT_Ingredients" (Variables|Default|GetIngredientId))
    (:then
      (bind _output_get (Variables|Default|SetIngredientData _returnvalue)))
    (:RowNotFound
      (bind _output_get_2 (Variables|Components|SetNameText 0))))
  (Rendering|Components|TextRender|SetText _output_get_2 (.DisplayName (Utilities|Struct|BreakS_IngredientData _output_get))))